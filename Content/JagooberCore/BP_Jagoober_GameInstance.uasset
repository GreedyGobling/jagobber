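; Game instance for Jagoober that owns the persistent audio settings save game and applies its volumes.
; On Init it creates a settings save object if none exists, then loads it from its slot, or writes it out if loading fails, and applies the volumes.
; Global, Music, FX and UI updaters set sound mix class overrides and cache values in the save object, which SaveSettings writes to disk.
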(event `self.ReceiveInit`
  (`KismetSystemLibrary.DelayUntilNextTick`)
  (bind _returnvalue (`GameplayStatics.DoesSaveGameExist` (`self.SettingsSaveGameSlot`)))
  (if (not _returnvalue)
    (bind _returnvalue_2 (`GameplayStatics.CreateSaveGameObject` "/Game/SaveGame/BP_SaveGame_Settings.BP_SaveGame_Settings_C"))
    (set `self.SettingsSaveGame` _returnvalue_2))
  (`self.LoadSettings`))

(fn `LoadSettings`
  (bind _settingssavegame (`self.SettingsSaveGame`))
  (`|ExecutionSequence`
    (:`then_0`
      (bind _returnvalue (`GameplayStatics.LoadGameFromSlot` (`self.SettingsSaveGameSlot`)))
      (bind _asbp_save_game_settings (cast `/Game/SaveGame/BP_SaveGame_Settings` _returnvalue)
        (:`then`
          (set `self.SettingsSaveGame` _asbp_save_game_settings))
        (:`CastFailed`
          (`GameplayStatics.SaveGameToSlot` (`self.SettingsSaveGame`) (`self.SettingsSaveGameSlot`)))))
    (:`then_1`
      (`self.UpdateGlobal` (`/Game/SaveGame/BP_SaveGame_Settings.Volume_Global` _settingssavegame))
      (`self.UpdateMusic` (`/Game/SaveGame/BP_SaveGame_Settings.Volume_Music` _settingssavegame))
      (`self.UpdateFX` (`/Game/SaveGame/BP_SaveGame_Settings.Volume_FX` _settingssavegame))
      (`self.UpdateUI` (`/Game/SaveGame/BP_SaveGame_Settings.Volume_UI` _settingssavegame)))))

(fn `SaveSettings`
  (bind _settingssavegame (`self.SettingsSaveGame`)
    (:`then`
      (`GameplayStatics.SaveGameToSlot` _settingssavegame (`self.SettingsSaveGameSlot`)))
    (:`else`)))

(fn `UpdateAudioSetting`
  (params (InSoundMixModifier :type "SoundMix Object Reference") (InSoundClass :type "SoundClass Object Reference") (Volume :type "Float (double-precision)"))
  (`GameplayStatics.SetSoundMixClassOverride` InSoundMixModifier InSoundClass Volume 1.0 0.0))

(fn `UpdateFX`
  (params (Volume :type "Float (double-precision)"))
  (`self.UpdateAudioSetting` "/Game/Audio/SoundMix/SCM_FX.SCM_FX" "/Game/Audio/SoundClass/SC_FX.SC_FX" Volume)
  (bind _settingssavegame (`self.SettingsSaveGame`)
    (:`then`
      (set `/Game/SaveGame/BP_SaveGame_Settings.Volume_FX` (`local.Volume`) _settingssavegame))
    (:`else`)))

(fn `UpdateGlobal`
  (params (Volume :type "Float (double-precision)"))
  (`self.UpdateAudioSetting` "/Game/Audio/SoundMix/SCM_Global.SCM_Global" "/Game/Audio/SoundClass/SC_Global.SC_Global" Volume)
  (bind _settingssavegame (`self.SettingsSaveGame`)
    (:`then`
      (set `/Game/SaveGame/BP_SaveGame_Settings.Volume_Global` (`local.Volume`) _settingssavegame))
    (:`else`)))

(fn `UpdateMusic`
  (params (Volume :type "Float (double-precision)"))
  (`self.UpdateAudioSetting` "/Game/Audio/SoundMix/SCM_Music.SCM_Music" "/Game/Audio/SoundClass/SC_Music.SC_Music" Volume)
  (bind _settingssavegame (`self.SettingsSaveGame`)
    (:`then`
      (set `/Game/SaveGame/BP_SaveGame_Settings.Volume_Music` (`local.Volume`) _settingssavegame))
    (:`else`)))

(fn `UpdateUI`
  (params (Volume :type "Float (double-precision)"))
  (`self.UpdateAudioSetting` "/Game/Audio/SoundMix/SCM_UI.SCM_UI" "/Game/Audio/SoundClass/SC_UI.SC_UI" Volume)
  (bind _settingssavegame (`self.SettingsSaveGame`)
    (:`then`
      (set `/Game/SaveGame/BP_SaveGame_Settings.Volume_UI` (`local.Volume`) _settingssavegame))
    (:`else`)))